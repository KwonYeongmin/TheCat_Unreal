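; BP_SH_Intro is a Paper2D flipbook Blueprint for the SH figure, apparently used in the game's intro.
; BeginPlay calls SetPlayerAnimation with index 0, a function not defined in this Blueprint.
; SetAnimation maps an index to a flipbook on MPPaperFlipbookComponent: idle by default, two intro variants, or an empty flipbook.
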(event EventBeginPlay
  (Class|CPlayerIntro|SetPlayerAnimation))

(fn ConstructionScript)

(fn SetAnimation
  (params (animIndex :type Integer))
  (bind _m_ppaperflipbookcomponent (Variables|Default|Getm_pPaperFlipbookComponent))
  (switch int animIndex
    (:Default
      _)
    (:0
      _)
    (:1
      (bind _returnvalue (Sprite|SetFlipbook _m_ppaperflipbookcomponent "/Game/Images/Intro/Characters/FlipBook/Intro_SH_FB_2.Intro_SH_FB_2"))
      (return _returnvalue))
    (:2
      (bind _returnvalue_2 (Sprite|SetFlipbook _m_ppaperflipbookcomponent "/Game/Images/Intro/Characters/FlipBook/Intro_SH_FB_1.Intro_SH_FB_1"))
      (return _returnvalue_2))
    (:3
      (bind _returnvalue_3 (Sprite|SetFlipbook _m_ppaperflipbookcomponent))
      (return _returnvalue_3)))
  (bind _returnvalue_4 (Sprite|SetFlipbook _m_ppaperflipbookcomponent "/Game/Images/Intro/Characters/FlipBook/Intro_SH_FB_Idle.Intro_SH_FB_Idle"))
  (return _returnvalue_4))