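; BP_SH is a player-controlled 2D flipbook character that walks horizontally along the world X axis.
; BeginPlay enables input and starts a looping flipbook, and the MoveRight axis drives movement input and records a Front facing flag.
; Each tick picks the walk or idle flipbook from velocity and mirrors the sprite by flipping its X scale with the direction of travel.
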(event Custom|UpdateAnimation
  ;[1 1 1] UpdateAnimation
  (Sprite|SetFlipbook (Variables|Default|Getm_pPaperFlipbookComponent) (select (> (Math|Vector|VectorLength (Variables|/Script/Engine.MovementComponent|GetVelocity (Variables|Character|GetCharacterMovement))) 0.0) "/Game/Images/Player/Flipbooks/Player_Walk_Flipbook.Player_Walk_Flipbook" "/Game/Images/Player/Flipbooks/Player_Idle_Flipbook.Player_Idle_Flipbook")))

(event Custom|UpdateRotation
  (bind _m_ppaperflipbookcomponent (Variables|Default|Getm_pPaperFlipbookComponent))
  ;[1 1 1] UpdateRotate
  (Utilities|IsValid (Pawn|GetController)
    (:Is%20Valid
      (Math|Float|CompareFloat (.X (Math|Vector|BreakVector (Variables|/Script/Engine.MovementComponent|GetVelocity (Variables|Character|GetCharacterMovement)))) 0.0
        (:>
          (Transformation|SetWorldScale3D _m_ppaperflipbookcomponent "0.650000,0.650000,0.650000"))
        (:<
          (Transformation|SetWorldScale3D _m_ppaperflipbookcomponent "-0.650000,0.650000,0.650000"))))))

(event EventBeginPlay
  (bind _m_ppaperflipbookcomponent (Variables|Default|Getm_pPaperFlipbookComponent))
  ;[1 1 1] BeginPlay
  (Input|EnableInput (Game|GetPlayerController 0))
  (Variables|Default|Setspeed 0.5)
  (Audio|Components|Audio|Play _m_ppaperflipbookcomponent)
  (Components|Timeline|SetLooping _m_ppaperflipbookcomponent true))

(event EventTick
  (params (DeltaSeconds :type Float%20%28single-precision%29))
  ;[1 1 1] Tick
  (CallFunction|UpdateAnimation)
  (CallFunction|UpdateRotation))

(event Input|AxisEvents|InputAxisMoveRight
  (params (AxisValue :type Float%20%28single-precision%29))
  ;[1 1 1] InputAxisMoveRight
  (Pawn|Input|AddMovementInput (Math|Vector|MakeVector (Variables|Default|Getspeed) 0.0 0.0) AxisValue false)
  (Variables|Default|SetbFront (> AxisValue 0.0)))

(fn ConstructionScript)